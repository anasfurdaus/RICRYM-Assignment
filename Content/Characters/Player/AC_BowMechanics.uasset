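; AC_BowMechanics is a player character component that handles entering and leaving bow aim.
; On BeginPlay it caches the owning Character and its initial movement rotation rate.
; AimBegin sets the aiming flag and makes the character turn toward the controller's desired rotation at a dedicated aim rate.
; AimEnd clears the flag, returns to orient-to-movement and restores the cached rate.
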(event `self.ReceiveBeginPlay`
  (bind _ascharacter (cast `Character` (`self.GetOwner`)))
  (set `self.CharacterRef` _ascharacter)
  (set `self.InitialRotationRate` (`CharacterMovementComponent.RotationRate` (`Character.CharacterMovement` (`self.CharacterRef`)))))

(event `AimBegin`
  (bind _charactermovement (`Character.CharacterMovement` (`self.CharacterRef`)))
  (set `self.IsAiming` true)
  (set `CharacterMovementComponent.bOrientRotationToMovement` false _charactermovement)
  (set `CharacterMovementComponent.bUseControllerDesiredRotation` true _charactermovement)
  (set `CharacterMovementComponent.RotationRate` (`self.AimRotationRate`) _charactermovement))

(event `AimEnd`
  (bind _charactermovement (`Character.CharacterMovement` (`self.CharacterRef`)))
  (set `self.IsAiming` false)
  (set `CharacterMovementComponent.bOrientRotationToMovement` true _charactermovement)
  (set `CharacterMovementComponent.bUseControllerDesiredRotation` false _charactermovement)
  (set `CharacterMovementComponent.RotationRate` (`self.InitialRotationRate`) _charactermovement))