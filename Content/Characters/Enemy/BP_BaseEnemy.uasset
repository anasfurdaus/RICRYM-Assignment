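; Base melee enemy character that attacks the player with a sword, takes damage and dies.
; Server-routed RPC attacks play a montage, while HitDetect sphere-traces at the sword socket to trigger the player's hit reaction.
; Hits play random impact montages and drain health; death flags the AI blackboard, plays a montage, destroys the actor, increments score and requests a GameMode respawn.
; Tick updates the health bar widget and turns it toward the camera.
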(event `RPC_Attack`
  ; Attack
  (bind _asbp_third_person_character (cast `/Game/ThirdPerson/Blueprints/BP_ThirdPersonCharacter` (`GameplayStatics.GetPlayerCharacter` 0)))
  (if (`NavMovementInterface.IsFalling` (`self.CharacterMovement`))
    _
    (elif (`self.Attacking`)
      _
      (elif (`self.isDeadNPC`)
        _
        (elif (not (`/Game/ThirdPerson/Blueprints/BP_ThirdPersonCharacter.isDead` _asbp_third_person_character))
          (set `self.Attacking` true)
          (`KismetSystemLibrary.PrintString` "Attacking")
          (`|PlayMontage` (`self.SkeletalMesh`) "/Game/Characters/Warrior/Attack.Attack"
            (:`OnCompleted`
              _)
            (:`OnInterrupted`
              _))
          (set `self.Attacking` false)
          (`self.OnAttackEnd`)
          (`KismetSystemLibrary.PrintString` "Enemy Done Attacking"))))))

(event `Attack`
  ; Attack
  (`self.RPC_Server_Attack` :!label _label))

(event `InputAction|Attack`
  (params (Key :type "Key Structure"))
  ; Attack
  (:`Pressed`
    (goto _label)))

(event `RPC_Server_Attack`
  ; Attack
  (`self.RPC_Attack`))

(event `Hit_React`
  ; Hit Reaction
  (if (not (`self.IsHit`))
    (set `self.IsHit` true)
    (`|PlayMontage` (`self.SkeletalMesh`) (select `int` (`KismetMathLibrary.RandomIntegerInRange` 0 1) :`0` "/Game/Characters/Warrior/Impact_1.Impact_1" :`1` "/Game/Characters/Warrior/Impact_2.Impact_2" :!type "AnimMontage Object Reference")
      (:`then`
        (bind _output_get (set `self.Health` (- (`self.Health`) 25.0)))
        (`KismetSystemLibrary.PrintString` (`KismetStringLibrary.Conv_DoubleToString` _output_get)))
      (:`OnCompleted`
        (set `self.IsHit` false :!label _label_2)
        (if (<= (`self.Health`) 0.0)
          (`|PlayMontage` (`self.SkeletalMesh`) (select `int` (`KismetMathLibrary.RandomIntegerInRange` 0 1) :`0` "/Game/Characters/Warrior/Death_1.Death_1" :`1` "/Game/Characters/Warrior/Death_2.Death_2" :!type "AnimMontage Object Reference")
            (:`then`
              (bind _output_get_2 (set `self.isDeadNPC` true))
              (bind _asbp_ai (cast `/Game/Characters/Enemy/AI/BP_AI` (`self.GetController`)))
              (`BlackboardComponent.SetValueAsBool` (`AIBlueprintHelperLibrary.GetBlackboard` _asbp_ai) (`self.isDead?`) _output_get_2))
            (:`OnCompleted`
              (`self.K2_DestroyActor` :!label _label_3)
              (bind _asbp_third_person_game_mode (cast `/Game/ThirdPerson/Blueprints/BP_ThirdPersonGameMode` (`GameplayStatics.GetGameMode`)))
              (bind _result (`/Engine/EditorBlueprintResources/StandardMacros.IncrementInt` (`/Game/ThirdPerson/Blueprints/BP_ThirdPersonGameMode.Score` _asbp_third_person_game_mode))
                (:`  `
                  (set `/Game/ThirdPerson/Blueprints/BP_ThirdPersonGameMode.Score` _result _asbp_third_person_game_mode))))
            (:`OnBlendOut`
              (goto _label_3)))))
      (:`OnInterrupted`
        (goto _label_2)))))

(event `self.ReceiveTick`
  (params (DeltaSeconds :type "Float (single-precision)"))
  (bind _healthbar (`self.HealthBar`))
  ; Healthbar
  (bind _aswb_health (cast `/Game/Characters/WB_Health` (`WidgetComponent.GetWidget` (`self.HealthBar`))))
  (`ProgressBar.SetPercent` (`/Game/Characters/WB_Health.Health_Bar` _aswb_health) (/ (`self.Health`) 100.0))
  (`SceneComponent.K2_SetWorldRotation` _healthbar (`KismetMathLibrary.FindLookAtRotation` (`SceneComponent.K2_GetComponentLocation` _healthbar) (`SceneComponent.K2_GetComponentLocation` (`PlayerCameraManager.TransformComponent` (`GameplayStatics.GetPlayerCameraManager` 0)))) false false))

(event `self.ReceiveDestroyed`
  ; Respawn
  (bind _asbp_third_person_game_mode (cast `/Game/ThirdPerson/Blueprints/BP_ThirdPersonGameMode` (`GameplayStatics.GetGameMode`)))
  (`/Game/ThirdPerson/Blueprints/BP_ThirdPersonGameMode.Respawn NPC` _asbp_third_person_game_mode))

(fn `Hit_Detect`
  (bind _returnvalue (`SceneComponent.GetSocketLocation` (`self.SkeletalMesh`) "Sword_joint"))
  (bind _outhit (`KismetSystemLibrary.SphereTraceSingleForObjects` :`Start` _returnvalue :`End` _returnvalue :`Radius` 60.0 :`ObjectTypes` (`|MakeArray` "ObjectTypeQuery3" :!type "EObjectTypeQuery Enum") :`DrawTime` 2.5))
  (bind _asbp_third_person_character (cast `/Game/ThirdPerson/Blueprints/BP_ThirdPersonCharacter` (`.HitActor` (`GameplayStatics.BreakHitResult` _outhit))))
  (`/Game/ThirdPerson/Blueprints/BP_ThirdPersonCharacter.Hit_React` _asbp_third_person_character)
  (`KismetSystemLibrary.PrintString` "Player is hit"))

(fn `UserConstructionScript`)